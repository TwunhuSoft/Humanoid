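; Game mode for a wave-based zombie game that starts spawning on BeginPlay and prints a win message after the final wave is cleared.
; Each wave's zombie count scales with the current wave number and is split between two spawn transforms.
; The ZombieKilled event counts down the remaining zombies and advances the wave at zero, spawning the next batch immediately without a delay.
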(event `self.ReceiveBeginPlay`
  ;[1 1 1] Start Game
  (`self.StartGame`))

(event `StartGame`
  ;[1 1 1] Start Game
  (`self.SpawnZombies`))

(event `SpawnZombies`
  ;[1 1 1] Sapwn the zombies
  (bind _output_get (set `self.ZombieTotal` (* (`self.CurrentWave`) 4)))
  (set `self.ZombiesLeft` _output_get)
  (for _index (range (+ _output_get 1))
    (if (== _index (/ (`self.ZombieTotal`) 2))
      (break)
      (else
        (`|SpawnActorFromClass` "/Game/_Main/Creatures/BP_Zombie.BP_Zombie_C" (`self.SpawnLocation1`) "Undefined" "OverrideRootScale" null null))))
  (for _ (range 1 (+ (/ (`self.ZombieTotal`) 2) 1))
    (`|SpawnActorFromClass` "/Game/_Main/Creatures/BP_Zombie.BP_Zombie_C" (`self.SpawnLocation2`) "Undefined" "OverrideRootScale" null null)))

(event `ZombieKilled`
  (bind _result (`/Engine/EditorBlueprintResources/StandardMacros.DecrementInt` (`self.ZombiesLeft`))
    (:`  `
      (if (== _result 0)
        (`self.WaveIncrement`)))))

(event `WaveIncrement`
  (if (== (`self.CurrentWave`) (`self.MaxWaves`))
    (`KismetSystemLibrary.PrintString` "You have won game")
    (else
      (`/Engine/EditorBlueprintResources/StandardMacros.IncrementInt` (`self.CurrentWave`)
        (:`  `
          (`self.SpawnZombies`)
          (`KismetSystemLibrary.PrintString` "Next Wave starting soon"))))))

(fn `UserConstructionScript`)